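; BP_SceneManager keeps a keyed map of scenes, tracks the current one and moves the player between them.
; GetScene looks up a scene by key, and GetCurrentScene returns the stored current key.
; UpdateScene, when the key is found, records it as current and sets the given player actor's transform to that scene's transform.
; The event graph and construction script hold no logic, so scene changes happen only when UpdateScene is called.
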(event EventBeginPlay)

(event Collision|EventActorBeginOverlap
  (params (OtherActor :type Actor%20Object%20Reference)))

(event EventTick
  (params (DeltaSeconds :type Float%20%28single-precision%29)))

(fn ConstructionScript)

(fn GetScene
  (params (Key :type E_Scene%20Enum :default "NewEnumerator0"))
  (bind _scenes (Variables|Default|GetScenes))
  (bind (_value _returnvalue) (Utilities|Map|Find _scenes Key))
  ;[1 1 1] Get scene based off key
  (return _value _returnvalue))

(fn GetCurrentScene
  ;[1 1 1] Get current scene
  (return (Variables|Default|GetCurrentScene)))

(fn UpdateScene
  (params (Player :type BP%20Player%20Object%20Reference) (Scene :type E_Scene%20Enum :default "NewEnumerator0"))
  (bind (_scene _found) (CallFunction|GetScene Scene))
  (if _found
    (Variables|Default|SetCurrentScene Scene)
    (Transformation|SetActorTransform Player (Default|GetSceneTransform _scene))))