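; BP_Guest is a bar guest NPC that orders a random drink and waits for it until its patience runs out.
; Clicking it places the order with the game mode and speaks a voiceline with the drink name filled in from the player's recipe book.
; Receiving a drink or timing out has the game mode resolve the order, stops interaction, and fires the guest-left delegate after a short delay.
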(event Custom|OrderExpired
  (CallFunction|ReceiveDrink false))

(event Custom|Leave
  (Default|CallGuestLeftDelegate self))

(event Custom|ReceiveDrink
  (params (Received :type Boolean) (Drink :type BP%20Drink%20Object%20Reference))
  (Default|ResolveOrder (CallFunction|GetGameModeRef) self Drink Received)
  (Variables|Default|SetAcceptingInteraction false)
  (Utilities|Time|SetTimerbyEvent (delegate Custom|Leave) 3.0))

(event EventBeginPlay
  (CallFunction|RandomizeOrder)
  (Utilities|Time|SetTimerbyEvent (delegate Custom|OrderExpired) (Variables|Default|GetPatience)))

(event EventClicked
  (params (Player :type BP%20Player%20Object%20Reference))
  (bind _order (CallFunction|GetOrder))
  (bind (_value _found) (CallFunction|GetVoiceline "NewEnumerator0"))
  (bind (_recipebook _valid) (Default|GetRecipeBook Player))
  (bind (_voiceline _duration _cps) (Utilities|Struct|BreakF_Voiceline _value))
  (bind (_recipe _found_2) (Default|GetRecipe _recipebook _order))
  (if (Variables|Default|GetAcceptingInteraction)
    (Utilities|IsValid (CallFunction|GetGameModeRef)
      (:Is%20Valid
        (Default|PlaceOrder (CallFunction|GetGameModeRef) self (CallFunction|GetOrder))
        (if (and _found _valid)
          (if _found_2
            (CallFunction|Talk (Utilities|Struct|MakeF_Voiceline (Utilities|String|Replace _voiceline "{drink}" (Utilities|String|ToString(Name) (Default|GetRecipeName _recipe)) "CaseSensitive") _duration _cps))))))))

(event Event
  (params (Actor :type Actor%20Object%20Reference))
  (if (Variables|Default|GetAcceptingInteraction)
    (bind _asbp_drink (Utilities|Casting|CastToBP_Drink Actor))
    (CallFunction|ReceiveDrink true _asbp_drink)))

(fn ConstructionScript
  (|CallParentFunction))

(fn RandomizeOrder
  ;[1 1 1] Randomize order
  (bind _output_get (Variables|Default|SetOrder (Utilities|Enum|ByteToEnumE_Drink (Math|Conversions|ToByte(Integer) (Math|Random|RandomIntegerinRange 0 (- (Math|Conversions|ToInteger(Byte) (Utilities|Enum|LiteralenumE_Drink "NewEnumerator1")) 1))))))
  (return _output_get))

(fn GetOrder
  ;[1 1 1] Get order
  (return (Variables|Default|GetOrder)))

(fn GetNPCType
  ;[1 1 1] Get NPC type
  (return "NewEnumerator0"))

(fn GetVoiceline
  (params (Key :type E_GuestVoiceline%20Enum :default "NewEnumerator0"))
  (bind _voicelines (Variables|Default|GetVoicelines))
  (bind (_value _returnvalue) (Utilities|Map|Find _voicelines Key))
  ;[1 1 1] Get voiceline
  (return _value _returnvalue))