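; BP_Garnish is a draggable 2D garnish item for the Fantasy Cocktails game.
; Drag has the player pick it up, raises the render component's translucent sort priority and plays a sound.
; Drop makes the player release it, then resets the item.
; Getters expose the garnish, its flipbook for when placed on the glass, and its socket name.
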(event EventBeginPlay
  (|CallParentFunction))

(event EventDrop
  (params (Player :type BP%20Player%20Object%20Reference))
  (Default|DropItem Player)
  (CallFunction|ResetItem))

(event EventDrag
  (params (Player :type BP%20Player%20Object%20Reference))
  (Default|PickupItem Player self)
  (Rendering|SetTranslucentSortPriority (Variables|Default|GetRenderComponent) 1)
  ;[1 1 1] Drag Sound
  (Audio|PlaySound2D (Variables|Default|GetSound) 1.0 1.0 0.0 0 0))

(fn ConstructionScript)

(fn GetGarnish
  ;[1 1 1] Get garnish
  (return (Variables|Default|GetGarnish)))

(fn GetPlacedFlipbook
  ;[1 1 1] Get placed flipbook (on the glass)
  (return (Variables|Default|GetPlacedFlipbook)))

(fn GetSocketName
  ;[1 1 1] Get socket name
  (return (Variables|Default|GetSocketName)))