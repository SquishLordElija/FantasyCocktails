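; Player controller Blueprint for FantasyCocktails that provides mouse-to-world picking helpers.
; GetHitResultFromMouse deprojects the cursor and line traces on Visibility over Distance along the camera's forward vector rather than the deprojected ray, writing the hit by reference and returning whether it struck.
; GetMouseWorldLocation returns the cursor's deprojected world position.
; The event graph holds no active logic.
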(event EventBeginPlay)

(event EventTick
  (params (DeltaSeconds :type Float%20%28single-precision%29)))

(fn ConstructionScript)

(fn GetHitResultfromMouse
  (params (Hit :type Hit%20Result%20Structure%20%28by%20ref%29))
  (bind (_locationx _locationy) (Game|Player|GetMousePosition))
  (bind _self self)
  (bind _returnvalue (Math|Vector2D|MakeVector2D _locationx _locationy))
  (bind _worldposition (Class|GameplayStatics|DeprojectScreentoWorld _self _returnvalue))
  ;[1 1 1] Line trace from the mouse
  (bind (_outhit _returnvalue_2) (Collision|LineTraceByChannel _worldposition (+ _worldposition (* (Math|Vector|GetForwardVector (Camera|GetCameraRotation (Variables|Default|GetPlayerCameraManager))) (LocalVariables|GetDistance))) "TraceTypeQuery1" false 0 "None"))
  (|SetBy-RefVar Hit _outhit)
  (return _returnvalue_2))

(fn GetMouseWorldLocation
  (bind (_locationx _locationy) (Game|Player|GetMousePosition))
  ;[1 1 1] Deproject mouse screen position to world location
  (return (.WorldPosition (Class|GameplayStatics|DeprojectScreentoWorld self (Math|Vector2D|MakeVector2D _locationx _locationy)))))