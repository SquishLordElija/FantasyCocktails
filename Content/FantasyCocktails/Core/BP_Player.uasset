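; Player for the cocktail bar game, handling mouse interaction, held items and containers, scene turning and drink tickets.
; Each tick a cursor trace finds the hover target, which input routes through clickable, draggable and recipient interfaces while held items follow the mouse.
; Shaker delegates swap the player's flipbook, with shaking also locking interaction and container dropping.
; It also creates and resets the current ticket and spawns drinks at free counter spots.
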(event Custom|SetupShaker
  (bind (_shaker _returnvalue) (CallFunction|GetShaker))
  ;[1 1 1] Update animations for shaker
  ;;[1 1 1] Shake
  (if _returnvalue
    (EventDispatchers|BindEventtoShakeDelegate _shaker (delegate Custom|Shaker_Shake))
    ;;[1 1 1] Strain
    (EventDispatchers|BindEventtoStrainDelegate (.Shaker (CallFunction|GetShaker)) (delegate Custom|Shaker_Strain))))

(event Custom|SetupInput
  (params (PlayerController :type Player%20Controller%20Object%20Reference) (MappingContext :type Input%20Mapping%20Context%20Object%20Reference))
  ;[1 1 1] Setup Input
  (Input|AddMappingContext (PlayerController|LocalPlayerSubsystems|GetEnhancedInputLocalPlayerSubsystem PlayerController) MappingContext 0 "(bIgnoreAllPressedKeysUntilRelease=True,bForceImmediately=False,bNotifyUserSettings=False)"))

(event Custom|RegisterGameMode
  ;[1 1 1] Set game mode reference
  (bind _asbp_bar_game_mode (Utilities|Casting|CastToBP_BarGameMode (Game|GetGameMode)))
  (Variables|Default|SetGameModeRef _asbp_bar_game_mode))

(event Custom|Shaker_Shake
  (params (Shaking :type Boolean))
  (bind _returnvalue (not Shaking))
  ;[1 1 1] Update animations for shaker
  ;;[1 1 1] Shake
  (Variables|Default|SetCanInteract _returnvalue)
  (Variables|Default|SetCanDropContainer _returnvalue)
  (CallFunction|UpdateFlipbook (select Shaking (Utilities|Enum|LiteralenumE_PlayerFlipbook "NewEnumerator2") (Utilities|Enum|LiteralenumE_PlayerFlipbook "NewEnumerator1"))))

(event Custom|RegisterPlayerController
  ;[1 1 1] Register player controller
  (bind _asbp_player_controller (Utilities|Casting|CastToBP_PlayerController (Pawn|GetController)))
  (Variables|Default|SetPlayerController _asbp_player_controller))

(event Custom|GameBegan
  ;[1 1 1] Setup
  ;;[1 1 1] Game Began
  (CallFunction|SetupInput (Variables|Default|GetPlayerController) "/Game/FantasyCocktails/Core/Input/IMC_Player.IMC_Player")
  (CallFunction|SetupShaker)
  (CallFunction|ResetTicket)
  (bind _returnvalue (UserInterface|CreateWidget "/Game/FantasyCocktails/Core/WBP_Identifier.WBP_Identifier_C" (Variables|Default|GetPlayerController) self))
  (UserInterface|Viewport|AddtoViewport _returnvalue 0)
  (Class|GameplayStatics|SetViewportMouseCaptureMode "CapturePermanently_IncludingInitialMouseDown"))

(event Custom|Shaker_Strain
  (params (Apply :type Boolean))
  ;[1 1 1] Update animations for shaker
  ;;[1 1 1] Strain
  (if (Default|IsHeld (.Shaker (CallFunction|GetShaker)))
    (CallFunction|UpdateFlipbook (select Apply (Utilities|Enum|LiteralenumE_PlayerFlipbook "NewEnumerator3") (Utilities|Enum|LiteralenumE_PlayerFlipbook "NewEnumerator1")))))

(event Input|EnhancedActionEvents|EnhancedInputActionIA_Interact
  (params (ActionValue :type Boolean) (ElapsedSeconds :type Float%20%28double-precision%29) (TriggeredSeconds :type Float%20%28double-precision%29) (InputAction :type Input%20Action%20Object%20Reference :default "/Game/FantasyCocktails/Core/Input/Actions/IA_Interact.IA_Interact"))
  (bind _mousehit (Variables|Default|GetMouseHit))
  (bind _helditem (Variables|Default|GetHeldItem))
  (bind _mousehit_2 (Variables|Default|GetMouseHit))
  (bind _mousehit_3 (Variables|Default|GetMouseHit))
  (bind _hitactor (Collision|BreakHitResult _mousehit_3))
  (bind _hitactor_2 (Collision|BreakHitResult _mousehit))
  (bind _hitactor_3 (Collision|BreakHitResult _mousehit_2))
  ;[1 1 1] Interaction
  (if (Variables|Default|GetCanInteract)
    (bind _output_get (Variables|Default|SetInteractKeyDown ActionValue))
    (if _output_get
      (if (Variables|Default|GetHovering)
        (Utilities|FlowControl|Sequence
          (:then_0
            ;[1 1 1] Click
            (if (Utilities|DoesObjectImplementInterface _hitactor_3 "/Game/FantasyCocktails/Core/BPI_Clickable.BPI_Clickable_C")
              (Class|BPIClickable|Clicked(Message) _hitactor_3 self)))
          (:then_1
            ;[1 1 1] Drag/Pickup
            (if (not (CallFunction|IsHoldingItem))
              (if (Utilities|DoesObjectImplementInterface _hitactor_2 "/Game/FantasyCocktails/Core/BPI_Draggable.BPI_Draggable_C")
                (Class|BPIDraggable|Drag(Message) _hitactor_2 self))))))
      (else
        ;;[1 1 1] Drop
        (if (CallFunction|IsHoldingItem)
          (if (Utilities|DoesObjectImplementInterface _helditem "/Game/FantasyCocktails/Core/BPI_Draggable.BPI_Draggable_C")
            (Utilities|FlowControl|Sequence
              (:then_0
                ;;;[1 1 1] Receive
                (if (Variables|Default|GetHovering)
                  (if (Utilities|DoesObjectImplementInterface _hitactor "/Game/FantasyCocktails/Core/BPI_Recipient.BPI_Recipient_C")
                    (Class|BPIRecipient|Receive(Message) _hitactor _helditem))))
              (:then_1
                (Class|BPIDraggable|Drop(Message) (Variables|Default|GetHeldItem) self)))))))))

(event Input|EnhancedActionEvents|EnhancedInputActionIA_DropContainer
  (params (ActionValue :type Boolean) (ElapsedSeconds :type Float%20%28double-precision%29) (TriggeredSeconds :type Float%20%28double-precision%29) (InputAction :type Input%20Action%20Object%20Reference :default "/Game/FantasyCocktails/Core/Input/Actions/IA_DropContainer.IA_DropContainer"))
  ;[1 1 1] Drop Container
  (CallFunction|DropContainer)
  (CallFunction|UpdateFlipbook "NewEnumerator0"))

(event Input|EnhancedActionEvents|EnhancedInputActionIA_Turn
  (params (ActionValue :type Boolean) (ElapsedSeconds :type Float%20%28double-precision%29) (TriggeredSeconds :type Float%20%28double-precision%29) (InputAction :type Input%20Action%20Object%20Reference :default "/Game/FantasyCocktails/Core/Input/Actions/IA_Turn.IA_Turn"))
  (bind _gamemoderef (Variables|Default|GetGameModeRef))
  (bind (_scenemanager _valid) (Default|GetSceneManager _gamemoderef))
  ;[1 1 1] Turn
  (if _valid
    (Default|UpdateScene _scenemanager self (Utilities|Select :Index (Default|GetCurrentScene _scenemanager) :NewEnumerator0 "NewEnumerator1" :NewEnumerator1 "NewEnumerator0" :NewEnumerator2 "NewEnumerator1"))))

(event Input|EnhancedActionEvents|EnhancedInputActionIA_Use
  (params (ActionValue :type Boolean) (ElapsedSeconds :type Float%20%28double-precision%29) (TriggeredSeconds :type Float%20%28double-precision%29) (InputAction :type Input%20Action%20Object%20Reference :default "/Game/FantasyCocktails/Core/Input/Actions/IA_Use.IA_Use"))
  (bind (_shaker _returnvalue) (CallFunction|GetShaker))
  ;[1 1 1] Use container in hand (only shaker for now)
  (if _returnvalue
    (if (not (Default|IsShaking _shaker))
      (if (not (CallFunction|IsHoldingItem))
        (Default|Shake _shaker)))))

(event Input|EnhancedActionEvents|EnhancedInputActionIA_Acknowledge
  (params (ActionValue :type Boolean) (ElapsedSeconds :type Float%20%28double-precision%29) (TriggeredSeconds :type Float%20%28double-precision%29) (InputAction :type Input%20Action%20Object%20Reference :default "/Game/FantasyCocktails/Core/Input/Actions/IA_Acknowledge.IA_Acknowledge"))
  (bind _gamemoderef (Variables|Default|GetGameModeRef))
  (bind (_tutorial _barmaid) (Default|IsTutorial _gamemoderef))
  (Utilities|IsValid (Variables|Default|GetGameModeRef)
    (:Is%20Valid
      (if _tutorial
        (Default|Conversate _barmaid)))))

(event EventBeginPlay
  ;[1 1 1] Setup
  (CallFunction|RegisterGameMode)
  ;;[1 1 1] Save default transform for item attach point
  (Variables|Default|SetAttachedItemDefaultTransform (Transformation|GetWorldTransform (Variables|Default|GetItemAttach)))
  ;;[1 1 1] Game Began
  (EventDispatchers|BindEventtoGameBeganDelegate (Variables|Default|GetGameModeRef) (delegate Custom|GameBegan))
  (CallFunction|RegisterPlayerController)
  (CallFunction|SetupInput (Variables|Default|GetPlayerController) "/Game/FantasyCocktails/Core/Input/IMC_Default.IMC_Default"))

(event EventTick
  (params (DeltaSeconds :type Float%20%28single-precision%29))
  (bind _array (Utilities|Array|MakeArray "ObjectTypeQuery2"))
  (bind _playercontroller (Variables|Default|GetPlayerController))
  (bind _playercontroller_2 (Variables|Default|GetPlayerController))
  (bind _newparam (Default|GetMouseWorldLocation _playercontroller))
  (bind (_hitresult _returnvalue) (Class|PlayerController|GetHitResultUnderCursorforObjects _playercontroller_2 _array true))
  ;[1 1 1] Hovering
  (Utilities|IsValid _playercontroller_2
    (:Is%20Valid
      (bind _output_get (Variables|Default|SetMouseHit _hitresult))
      (bind _output_get_2 (Variables|Default|SetHovering _returnvalue))
      ;[1 1 1] Drag
      (if _output_get_2
        (Utilities|IsValid (.HitActor (Collision|BreakHitResult _output_get))
          (:Is%20Valid
            (Default|CallHoverTargetUpdated (.HitActor (Collision|BreakHitResult _output_get))))
          (:Is%20Not%20Valid
            _)))
      (if (CallFunction|IsHoldingItem)
        (Transformation|SetWorldLocation (Variables|Default|GetItemAttach) (Math|Vector|MakeVector 0.0 (.y _newparam) (.z _newparam)) false false)))))

(fn ConstructionScript)

(fn GetRecipeBook
  (bind _recipebook (Variables|Default|GetRecipeBook))
  ;[1 1 1] Get recipe book
  (return _recipebook (Utilities|IsValid _recipebook)))

(fn GetShaker
  (bind _shaker (Variables|Default|GetShaker))
  ;[1 1 1] Get shaker
  (return _shaker (Utilities|IsValid _shaker)))

(fn PickupItem
  (params (Actor :type Actor%20Object%20Reference))
  ;[1 1 1] Manually set actor location to account for pivot points
  (Transformation|SetActorLocation Actor (- (Transformation|GetActorLocation Actor) (.Origin (Collision|GetActorBounds Actor false false))) false false)
  ;[1 1 1] Attach item and set reference
  (Transformation|AttachComponentToComponent Actor (Variables|Default|GetItemAttach) "None" "KeepRelative" "KeepRelative" "KeepRelative" false)
  (bind _output_get (Variables|Default|SetHeldItem Actor))
  (Collision|SetActorEnableCollision _output_get false))

(fn DropItem
  ;[1 1 1] Detach held item
  (if (CallFunction|IsHoldingItem)
    (Transformation|DetachFromActor (Variables|Default|GetHeldItem) "KeepRelative" "KeepRelative" "KeepRelative")
    ;[1 1 1] Reset held item & attach point transform
    (Collision|SetActorEnableCollision (Variables|Default|GetHeldItem) true)
    (Variables|Default|SetHeldItem 0)
    (Transformation|SetWorldTransform (Variables|Default|GetItemAttach) (Variables|Default|GetAttachedItemDefaultTransform) false false)))

(fn UpdateFlipbook
  (params (Key :type E_PlayerFlipbook%20Enum :default "NewEnumerator0"))
  (bind _flipbooks (Variables|Default|GetFlipbooks))
  (bind (_value _returnvalue) (Utilities|Map|Find _flipbooks Key))
  ;[1 1 1] Update flipbook based on key
  (if _returnvalue
    (bind _returnvalue_2 (Sprite|SetFlipbook (Variables|Default|GetSprite) _value))
    (return _returnvalue_2)
    (else
      (return false))))

(fn IsHoldingItem
  ;[1 1 1] Return if held item is set
  (return (Utilities|IsValid (Variables|Default|GetHeldItem))))

(fn PickupContainer
  (params (Container :type BP%20Container%20Object%20Reference))
  (Transformation|AttachComponentToComponent Container (Variables|Default|GetContainerAttach) "None" "SnapToTarget" "KeepRelative" "KeepRelative" false)
  (Variables|Default|SetHeldContainer Container))

(fn IsHoldingContainer
  ;[1 1 1] Return true if held container is valid
  (return (Utilities|IsValid (Variables|Default|GetHeldContainer))))

(fn DropContainer
  ;[1 1 1] Detach container
  (if (CallFunction|IsHoldingContainer)
    (Transformation|DetachFromActor (Variables|Default|GetHeldContainer) "KeepRelative" "KeepRelative" "KeepRelative")
    ;[1 1 1] Reset container and dereference it
    (Default|Reset (Variables|Default|GetHeldContainer))
    (Variables|Default|SetHeldContainer 0)
    (CallFunction|UpdateFlipbook "NewEnumerator0")))

(fn GetCurrentTicket
  (bind _currentticket (Variables|Default|GetCurrentTicket))
  ;[1 1 1] Get ticket
  (return _currentticket (Utilities|IsValid _currentticket)))

(fn SpawnDrink
  (bind _ticket (CallFunction|GetCurrentTicket))
  (bind _gamemoderef (Variables|Default|GetGameModeRef))
  (bind (_drinkcounter _valid) (Default|GetDrinkCounter _gamemoderef))
  (if _valid
    (bind (_queue _found) (Default|Find _drinkcounter))
    (if _found
      (Default|Solidify _ticket)
      (bind _returnvalue (Game|SpawnActorfromClass "/Game/FantasyCocktails/Core/BP_Drink.BP_Drink_C" (Default|GetQueueTransform _queue) "Undefined" "MultiplyWithRoot" 0 _ticket (.RecipeBook (CallFunction|GetRecipeBook)) _queue 0))
      (Default|Occupy _queue)
      (return _returnvalue true)
      (else
        (return 0 false)))
    (else
      (return 0 false))))

(fn NewTicket
  (params (Shaker :type BP%20Shaker%20Object%20Reference) (Glass :type BP%20Glass%20Object%20Reference) (Garnish :type E_Garnish%20Enum :default "NewEnumerator1") (Flair :type E_Flair%20Enum :default "NewEnumerator1"))
  (bind _returnvalue (Game|ConstructObjectfromClass "/Game/FantasyCocktails/Core/BP_Ticket.BP_Ticket_C" Shaker Glass Garnish Flair))
  (return _returnvalue))

(fn ResetTicket
  (bind (_ticket _valid) (CallFunction|GetCurrentTicket))
  (bind _shaker (CallFunction|GetShaker))
  (bind (_glass _valid_2) (Default|GetGlass _ticket))
  (if _valid
    (Default|Solidify _ticket)
    (if _valid_2
      (Default|Reset _glass)
      (Default|Empty _glass)))
  (CallFunction|DropContainer)
  (Default|Reset _shaker)
  (Default|Empty _shaker)
  (bind _ticket_2 (CallFunction|NewTicket (.Shaker (CallFunction|GetShaker)) 0 "NewEnumerator1" "NewEnumerator1"))
  (Variables|Default|SetCurrentTicket _ticket_2))