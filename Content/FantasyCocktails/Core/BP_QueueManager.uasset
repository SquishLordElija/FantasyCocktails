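; Queue manager for Fantasy Cocktails that holds an array of queue positions, treated as seats, and looks up free ones.
; Find loops over the array and returns the first position whose IsOccupied check is false, with a flag for whether one was found.
; GetQueue exposes the whole array, which this Blueprint's graphs never fill or modify.
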(event EventBeginPlay)

(fn ConstructionScript)

(fn Find
  ;[1 1 1] Find first unoccupied seat
  (if (Utilities|Array|IsNotEmpty (Variables|Default|GetQueue))
    (bind _array_element (Utilities|Array|ForEachLoopwithBreak (Variables|Default|GetQueue) :!label _label)
      (:LoopBody
        (if (not (Default|IsOccupied _array_element))
          (LocalVariables|SetFoundPos _array_element)
          (goto _label Break)))
      (:Completed
        (return (LocalVariables|GetFoundPos) (Utilities|IsValid (LocalVariables|GetFoundPos)))))
    (else
      (return 0 false))))

(fn GetQueue
  ;[1 1 1] Get queue
  (return (Variables|Default|GetQueue)))