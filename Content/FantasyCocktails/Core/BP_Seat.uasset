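; BP_Seat is a seat in the Fantasy Cocktails game that holds a reference to an NPC, presumably its occupant.
; It exposes a simple getter and setter for that NPC variable.
; It has no active event logic, and its construction script only calls the parent.
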(event EventBeginPlay
  (|CallParentFunction) ; This node is disabled and will not be called.\nDrag off pins to build functionality.
)

(event Collision|EventActorBeginOverlap
  (params (OtherActor :type Actor%20Object%20Reference))
  (|CallParentFunction OtherActor) ; This node is disabled and will not be called.\nDrag off pins to build functionality.
)

(event EventTick
  (params (DeltaSeconds :type Float%20%28single-precision%29))
  (|CallParentFunction DeltaSeconds) ; This node is disabled and will not be called.\nDrag off pins to build functionality.
)

(fn ConstructionScript
  (|CallParentFunction))

(fn GetNPC
  ;[1 1 1] Get NPC
  (return (Variables|Default|GetNPC)))

(fn SetNPC
  (params (NPC :type BP%20NPC%20Object%20Reference))
  (Variables|Default|SetNPC NPC))