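; Game mode for a fantasy cocktail bar that runs the barmaid tutorial, the guest cycle, orders, reputation and game end.
; It caches the level's managers, seats the barmaid, then spawns random guests one after another until the guest limit.
; Orders are mapped per guest and resolved by drink type and quality, with results broadcast through delegates to adjust reputation.
; Every reputation update fires the game-ended delegate without a threshold check.
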(event Custom|OrderResolved
  (params (Guest :type BP%20NPC%20Object%20Reference) (Order :type E_Drink%20Enum :default "NewEnumerator2") (Quality :type E_Quality%20Enum :default "NewEnumerator0") (Incorrect :type Boolean) (Expired :type Boolean))
  (if Expired
    (CallFunction|UpdateReputation "NewEnumerator2" -20)
    (else
      (CallFunction|UpdateReputation Quality))))

(event Custom|ReputationUpdated
  (params (Reputation :type Integer))
  (Default|CallGameEndedDelegate "NewEnumerator0"))

(event Custom|GuestLeft
  (params (Guest :type BP%20Guest%20Object%20Reference))
  ;[1 1 1] Vacate occupied seat & destroy
  (bind (_seat _found) (Default|FindfromNPC (.SeatManager (CallFunction|GetSeatManager)) Guest))
  (if _found
    (Default|Vacate _seat)
    (Default|SetNPC _seat)
    (Actor|DestroyActor Guest)
    (if (>= (Variables|Default|GetGuestCounter) (Variables|Default|GetMaxGuests))
      (CallFunction|EndGame "NewEnumerator2")
      (else
        (CallFunction|NewGuest)))))

(event Custom|NewGuest
  (bind (_guest _spawned) (CallFunction|SpawnGuest))
  (if _spawned
    (EventDispatchers|BindEventtoGuestLeftDelegate _guest (delegate Custom|GuestLeft))
    (Math|Integer|IncrementInt (Variables|Default|GetGuestCounter))))

(event Custom|EndGame
  (params (Reason :type E_GameEndReason%20Enum :default "NewEnumerator0"))
  (Default|CallGameEndedDelegate Reason))

(event Custom|BeginTutorial
  (bind (_seat _found) (Default|FindSeat (Variables|Default|GetSeatManager)))
  (if _found
    (bind _returnvalue (Game|SpawnActorfromClass "/Game/FantasyCocktails/Core/BP_Barmaid.BP_Barmaid_C" (Default|GetQueueTransform _seat) "Undefined" "MultiplyWithRoot" 0 self _seat 0))
    (Default|Occupy _seat)
    (Default|SetNPC _seat _returnvalue)
    (bind _output_get (Variables|Default|SetBarmaidRef _returnvalue))
    (EventDispatchers|BindEventtoTutorialBeganDelegate _output_get (delegate Custom|BeganTutorial))
    (Default|BeginTutorial _output_get)
    (EventDispatchers|BindEventtoTutorialEndedDelegate _returnvalue (delegate Custom|TutorialEnded))))

(event Custom|BeganTutorial
  (Variables|Default|SetTutorial true))

(event Custom|TutorialEnded
  (Variables|Default|SetTutorial false)
  (Default|CallGameBeganDelegate)
  (bind _seat (Default|FindfromNPC (.SeatManager (CallFunction|GetSeatManager)) (Variables|Default|GetBarmaidRef)))
  (Default|Vacate _seat)
  (Actor|DestroyActor (Variables|Default|GetBarmaidRef))
  (CallFunction|NewGuest))

(event EventBeginPlay
  (CallFunction|RegisterItemManager)
  (CallFunction|RegisterSeatManager)
  (CallFunction|RegisterDrinkCounter)
  (CallFunction|RegisterSceneManager)
  (EventDispatchers|BindEventtoOrderResolvedDelegate (delegate Custom|OrderResolved))
  (EventDispatchers|BindEventtoReputationUpdatedDelegate (delegate Custom|ReputationUpdated))
  (CallFunction|BeginTutorial))

(fn ConstructionScript)

(fn RegisterItemManager
  (bind _returnvalue (Actor|GetActorOfClass "/Game/FantasyCocktails/Core/BP_ItemManager.BP_ItemManager_C"))
  (Variables|Default|SetItemManager _returnvalue))

(fn RegisterSeatManager
  (bind _returnvalue (Actor|GetActorOfClass "/Game/FantasyCocktails/Core/BP_SeatManager.BP_SeatManager_C"))
  (Variables|Default|SetSeatManager _returnvalue))

(fn RegisterDrinkCounter
  (bind _returnvalue (Actor|GetActorOfClass "/Game/FantasyCocktails/Core/BP_DrinkCounter.BP_DrinkCounter_C"))
  (Variables|Default|SetDrinkCounter _returnvalue))

(fn RegisterSceneManager
  (bind _returnvalue (Actor|GetActorOfClass "/Game/FantasyCocktails/Core/BP_SceneManager.BP_SceneManager_C"))
  (Variables|Default|SetSceneManager _returnvalue))

(fn GetItemManager
  (bind _itemmanager (Variables|Default|GetItemManager))
  ;[1 1 1] Return item manager and if its valid
  (return _itemmanager (Utilities|IsValid _itemmanager)))

(fn GetSeatManager
  (bind _seatmanager (Variables|Default|GetSeatManager))
  ;[1 1 1] Return seat manager and if its valid
  (return _seatmanager (Utilities|IsValid _seatmanager)))

(fn GetDrinkCounter
  (bind _drinkcounter (Variables|Default|GetDrinkCounter))
  ;[1 1 1] Return drink counter and if its valid
  (return _drinkcounter (Utilities|IsValid _drinkcounter)))

(fn GetSceneManager
  (bind _scenemanager (Variables|Default|GetSceneManager))
  ;[1 1 1] Return scene manager if valid
  (return _scenemanager (Utilities|IsValid _scenemanager)))

(fn SpawnGuest
  (bind (_seatmanager _valid) (CallFunction|GetSeatManager))
  ;[1 1 1] Spawn a guest if there's a vacant seat
  (if _valid
    (bind (_seat _found) (Default|FindSeat _seatmanager))
    (if _found
      (if (not (Default|IsOccupied _seat))
        (bind _returnvalue (Game|SpawnActorfromClass (CallFunction|GetRandomGuestClass) (Default|GetQueueTransform _seat) "Undefined" "MultiplyWithRoot" 0 self _seat 0))
        (Default|Occupy _seat)
        (Default|SetNPC _seat _returnvalue)
        (Utilities|Array|Add (Variables|Default|GetGuests) _returnvalue)
        (return _returnvalue true)
        (else
          (return 0 false)))
      (else
        (return 0 false)))
    (else
      (return 0 false))))

(fn GetGuests
  ;[1 1 1] Get guests
  (return (Variables|Default|GetGuests)))

(fn PlaceOrder
  (params (Guest :type BP%20Guest%20Object%20Reference) (Order :type E_Drink%20Enum :default "NewEnumerator0"))
  ;[1 1 1] Add order to map and call delegate
  (bind _found (CallFunction|GetOrder Guest))
  (if (not _found)
    (Utilities|Map|Add (Variables|Default|GetOrders) Guest Order)
    (Default|CallOrderPlacedDelegate Guest Order)))

(fn ResolveOrder
  (params (Guest :type BP%20Guest%20Object%20Reference) (Drink :type BP%20Drink%20Object%20Reference) (Expired :type Boolean))
  (if Expired
    (Utilities|Map|Remove (Variables|Default|GetOrders) Guest)
    (Default|CallOrderResolvedDelegate Guest "NewEnumerator2" "NewEnumerator2" false Expired)
    (Default|Delete Drink :!label _label)
    (else
      (bind (_order _found) (CallFunction|GetOrder Guest))
      (if _found
        (if (Utilities|Enum|Equal(Enum) _order (Default|GetDrinkType Drink))
          (Utilities|Map|Remove (Variables|Default|GetOrders) Guest)
          (Default|CallOrderResolvedDelegate Guest (Default|GetDrinkType Drink) (Default|GetQuality Drink) false Expired)
          (goto _label)
          (else
            (Utilities|Map|Remove (Variables|Default|GetOrders) Guest)
            (Default|CallOrderResolvedDelegate Guest (Default|GetDrinkType Drink) "NewEnumerator2" true Expired)
            (goto _label)))))))

(fn GetOrder
  (params (Guest :type BP%20Guest%20Object%20Reference))
  (bind _orders (Variables|Default|GetOrders))
  (bind (_value _returnvalue) (Utilities|Map|Find _orders Guest))
  (return _value _returnvalue))

(fn GetReputation
  ;[1 1 1] Get reputation
  (return (Variables|Default|GetReputation)))

(fn UpdateReputation
  (params (Quality :type E_Quality%20Enum :default "NewEnumerator0") (Override :type Integer))
  ;[1 1 1] Update reputation based on order quality
  (if (!= Override 0)
    (bind _output_get (Variables|Default|SetReputation (+ (Variables|Default|GetReputation) Override)))
    (Default|CallReputationUpdatedDelegate _output_get)
    (else
      (bind _output_get_2 (Variables|Default|SetReputation (Math|Integer|Clamp(Integer) (+ (Variables|Default|GetReputation) (Utilities|Select :Index Quality :NewEnumerator0 (LocalVariables|GetPerfect) :NewEnumerator1 (LocalVariables|GetGood) :NewEnumerator2 (LocalVariables|GetPoor))) 0 (+ (Variables|Default|GetReputation) (Utilities|Select :Index Quality :NewEnumerator0 (LocalVariables|GetPerfect) :NewEnumerator1 (LocalVariables|GetGood) :NewEnumerator2 (LocalVariables|GetPoor))))))
      (Default|CallReputationUpdatedDelegate _output_get_2))))

(fn GetRandomGuestClass
  ;[1 1 1] Get random guest class from array
  (return (.OutItem (Utilities|Array|Random (Variables|Default|GetGuestClasses)))))

(fn IsTutorial
  (return (Variables|Default|GetTutorial) (Variables|Default|GetBarmaidRef)))