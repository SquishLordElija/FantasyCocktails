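; Ticket for a cocktail-making game that holds the shaker, glass, garnish and flair of a drink and grades it against a recipe.
; EvaluateQuality sums faults from shaker and glass comparisons plus glass type and garnish mismatches, then maps the clamped total to three quality tiers, ignoring flair.
; ResetTicket resets garnish and flair, clears the glass and fires a reset delegate, leaving the shaker untouched.
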(fn GetShaker
  ;[1 1 1] Get shaker
  (return (Variables|Default|GetShaker)))

(fn GetGlass
  ;[1 1 1] Get glass
  (return (Variables|Default|GetGlass)))

(fn GetGarnish
  ;[1 1 1] Get garnish
  (return (Variables|Default|GetGarnish)))

(fn SetShaker
  (params (Shaker :type BP%20Shaker%20Object%20Reference))
  (Variables|Default|SetShaker Shaker))

(fn SetGarnish
  (params (Garnish :type E_Garnish%20Enum :default "NewEnumerator0"))
  (Variables|Default|SetGarnish Garnish))

(fn GetFlair
  ;[1 1 1] Get flair
  (return (Variables|Default|GetFlair)))

(fn SetFlair
  (params (Flair :type E_Flair%20Enum :default "NewEnumerator1"))
  (Variables|Default|SetFlair Flair))

(fn SetGlass
  (params (Glass :type BP%20Glass%20Object%20Reference))
  (Variables|Default|SetGlass Glass))

(fn EvaluateQuality
  (params (Recipe :type BP%20Recipe%20Object%20Reference))
  (bind _faults (Default|Compareto (Variables|Default|GetShaker) Recipe))
  (bind _faults_2 (Default|Compareto (Variables|Default|GetGlass) Recipe))
  (return (Utilities|Select :Index (Math|Integer|Clamp(Integer) (+ _faults_2 _faults (+ (Math|Conversions|ToInteger(Boolean) (Utilities|Enum|NotEqual(Enum) (Default|GetGlassType (Variables|Default|GetGlass)) (Default|GetGlass Recipe))) (Math|Conversions|ToInteger(Boolean) (Utilities|Enum|NotEqual(Enum) (Variables|Default|GetGarnish) (Default|GetGarnish Recipe))))) 0 3) :Option%200 "NewEnumerator0" :Option%201 "NewEnumerator1" :Option%202 "NewEnumerator1" :Option%203 "NewEnumerator2") (+ _faults_2 _faults (+ (Math|Conversions|ToInteger(Boolean) (Utilities|Enum|NotEqual(Enum) (Default|GetGlassType (Variables|Default|GetGlass)) (Default|GetGlass Recipe))) (Math|Conversions|ToInteger(Boolean) (Utilities|Enum|NotEqual(Enum) (Variables|Default|GetGarnish) (Default|GetGarnish Recipe)))))))

(fn ResetTicket
  (CallFunction|SetGarnish "NewEnumerator1")
  (CallFunction|SetFlair "NewEnumerator1")
  (CallFunction|SetGlass)
  (Default|CallTicketResetDelegate))