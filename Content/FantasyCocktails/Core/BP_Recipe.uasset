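; BP_Recipe holds the data for a cocktail recipe: ingredients, instructions, glass, garnish and flair.
; Ingredient and instruction getters switch on a type to return either the shaker or the glass list.
; A flipbook getter looks up a flipbook by glass type in a map and reports whether it was found, while simple getters expose the other fields.
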(fn GetIngredients
  (params (Type :type E_ContainerType%20Enum :default "NewEnumerator0"))
  ;[1 1 1] Get ingredients array based on type
  (switch Utilities|FlowControl|Switch|SwitchonE_ContainerType Type
    (:NewEnumerator0
      (return (Variables|Default|GetShakerIngredients)))
    (:NewEnumerator1
      (return (Variables|Default|GetGlassIngredients)))))

(fn GetInstructions
  (params (Type :type E_ContainerType%20Enum :default "NewEnumerator0"))
  ;[1 1 1] Get instructions
  (switch Utilities|FlowControl|Switch|SwitchonE_ContainerType Type
    (:NewEnumerator0
      (return (Variables|Default|GetShakerInstructions)))
    (:NewEnumerator1
      (return (Variables|Default|GetGlassInstructions)))))

(fn GetFlipbook
  (params (Glass :type E_Glass%20Enum :default "NewEnumerator0"))
  (bind _flipbooks (Variables|Default|GetFlipbooks))
  (bind (_value _returnvalue) (Utilities|Map|Find _flipbooks Glass))
  ;[1 1 1] Get flipbook from map based on the glass type
  (return _value _returnvalue))

(fn GetGlass
  ;[1 1 1] Get glass
  (return (Variables|Default|GetGlass)))

(fn GetGarnish
  ;[1 1 1] Get garnish
  (return (Variables|Default|GetGarnish)))

(fn GetFlair
  ;[1 1 1] Get flair
  (return (Variables|Default|GetFlair)))