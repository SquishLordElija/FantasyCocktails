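; Clickable recipe book for the cocktail game that defines every drink recipe and shows them in a widget.
; BeginPlay creates WBP_RecipeBook and builds hard-coded BP_Recipe objects, including a Sludge entry without ingredients, into a map keyed by drink type.
; Each recipe holds ingredients, instructions, garnish, glass, flair and per-glass flipbooks.
; Clicking opens and sets up the widget, while GetRecipe and GetRecipes expose the map for lookups.
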(event EventBeginPlay
  (bind _returnvalue (UserInterface|CreateWidget "/Game/FantasyCocktails/Core/WBP_RecipeBook.WBP_RecipeBook_C" (Game|GetPlayerController 0) self))
  (Variables|Default|SetRecipeBookWidget _returnvalue)
  ;[0.1927 0.1925 0.1717] Frog Eye Martini
  (CallFunction|NewRecipe "NewEnumerator0" (Utilities|Array|MakeArray "NewEnumerator0" "NewEnumerator2" "NewEnumerator4" "NewEnumerator3") "NewEnumerator0" "NewEnumerator0" "NewEnumerator0" (Utilities|Array|MakeArray "NewEnumerator0" "NewEnumerator1") "NewEnumerator0" (Utilities|Map|MakeMap "NewEnumerator0" "/Game/FantasyCocktails/Assets/Back/Flipbooks/Drinks/FrogMartini/PF_MartiniGray.PF_MartiniGray" "NewEnumerator1" "/Game/FantasyCocktails/Assets/Back/Flipbooks/Drinks/FrogMartini/PF_RocksGray.PF_RocksGray" "NewEnumerator2" "/Game/FantasyCocktails/Assets/Back/Flipbooks/Drinks/FrogMartini/PF_HurricaneGray.PF_HurricaneGray" "NewEnumerator3" "/Game/FantasyCocktails/Assets/Back/Flipbooks/Drinks/FrogMartini/PF_CollinsGray.PF_CollinsGray" "NewEnumerator4" "/Game/FantasyCocktails/Assets/Back/Flipbooks/Drinks/FrogMartini/PF_CoupeGray.PF_CoupeGray" "NewEnumerator5" "/Game/FantasyCocktails/Assets/Back/Flipbooks/Drinks/PF_MuleDrink.PF_MuleDrink") "NewEnumerator1" "Frog Eye Martini" "/Game/FantasyCocktails/Assets/Back/Sprites/Drinks/FrogMartini/SP_MartiniGray.SP_MartiniGray")
  ;[0.4171 0.1094 1] Floating Iced Tea
  (CallFunction|NewRecipe "NewEnumerator3" (Utilities|Array|MakeArray "NewEnumerator0" "NewEnumerator8" "NewEnumerator6" "NewEnumerator9" "NewEnumerator5" "NewEnumerator3") (Utilities|Array|MakeArray "NewEnumerator14" "NewEnumerator3") "NewEnumerator2" "NewEnumerator3" (Utilities|Array|MakeArray "NewEnumerator0" "NewEnumerator1") "NewEnumerator0" (Utilities|Map|MakeMap "NewEnumerator0" "/Game/FantasyCocktails/Assets/Back/Flipbooks/Drinks/FloatingIcedTea/PF_MartiniPurple.PF_MartiniPurple" "NewEnumerator1" "/Game/FantasyCocktails/Assets/Back/Flipbooks/Drinks/FloatingIcedTea/PF_RockPurple.PF_RockPurple" "NewEnumerator2" "/Game/FantasyCocktails/Assets/Back/Flipbooks/Drinks/FloatingIcedTea/PF_HurricanePurple.PF_HurricanePurple" "NewEnumerator3" "/Game/FantasyCocktails/Assets/Back/Flipbooks/Drinks/FloatingIcedTea/PF_CollinsPurple.PF_CollinsPurple" "NewEnumerator4" "/Game/FantasyCocktails/Assets/Back/Flipbooks/Drinks/FloatingIcedTea/PF_CoupePurple.PF_CoupePurple" "NewEnumerator5" "/Game/FantasyCocktails/Assets/Back/Flipbooks/Drinks/PF_MuleDrink.PF_MuleDrink") "NewEnumerator1" "Floating Iced Tea" "/Game/FantasyCocktails/Assets/Back/Sprites/Drinks/FloatingIcedTea/SP_CollinsPurple.SP_CollinsPurple")
  ;[1 0.3053 0] Sunset
  (CallFunction|NewRecipe "NewEnumerator4" (Utilities|Array|MakeArray "NewEnumerator7" "NewEnumerator21" "NewEnumerator3") (Utilities|Array|MakeArray "NewEnumerator15" "NewEnumerator3") "NewEnumerator3" "NewEnumerator2" (Utilities|Array|MakeArray "NewEnumerator0" "NewEnumerator1") "NewEnumerator0" (Utilities|Map|MakeMap "NewEnumerator0" "/Game/FantasyCocktails/Assets/Back/Flipbooks/Drinks/Sunset/PF_MartiniOrange.PF_MartiniOrange" "NewEnumerator1" "/Game/FantasyCocktails/Assets/Back/Flipbooks/Drinks/Sunset/PF_RocksOrange.PF_RocksOrange" "NewEnumerator2" "/Game/FantasyCocktails/Assets/Back/Flipbooks/Drinks/Sunset/PF_HurricaneOrange.PF_HurricaneOrange" "NewEnumerator3" "/Game/FantasyCocktails/Assets/Back/Flipbooks/Drinks/Sunset/PF_CollinsOrange.PF_CollinsOrange" "NewEnumerator4" "/Game/FantasyCocktails/Assets/Back/Flipbooks/Drinks/Sunset/PF_CoupeOrange.PF_CoupeOrange" "NewEnumerator5" "/Game/FantasyCocktails/Assets/Back/Flipbooks/Drinks/PF_MuleDrink.PF_MuleDrink") "NewEnumerator1" "Sunset" "/Game/FantasyCocktails/Assets/Back/Sprites/Drinks/Sunset/SP_HurricaneOrange.SP_HurricaneOrange")
  ;[0 0.5638 1] Igloo Mule
  (CallFunction|NewRecipe "NewEnumerator5" (Utilities|Array|MakeArray "NewEnumerator0" "NewEnumerator9" "NewEnumerator11") (Utilities|Array|MakeArray "NewEnumerator12" "NewEnumerator3") "NewEnumerator4" "NewEnumerator5" (Utilities|Array|MakeArray "NewEnumerator0") "NewEnumerator0" (Utilities|Map|MakeMap "NewEnumerator0" "/Game/FantasyCocktails/Assets/Back/Flipbooks/Drinks/IglooMule/PF_MartiniBlue.PF_MartiniBlue" "NewEnumerator1" "/Game/FantasyCocktails/Assets/Back/Flipbooks/Drinks/IglooMule/PF_RocksBlue.PF_RocksBlue" "NewEnumerator2" "/Game/FantasyCocktails/Assets/Back/Flipbooks/Drinks/IglooMule/PF_HurricaneBlue.PF_HurricaneBlue" "NewEnumerator3" "/Game/FantasyCocktails/Assets/Back/Flipbooks/Drinks/IglooMule/PF_CollinsBlue.PF_CollinsBlue" "NewEnumerator4" "/Game/FantasyCocktails/Assets/Back/Flipbooks/Drinks/IglooMule/PF_CoupeBlue.PF_CoupeBlue" "NewEnumerator5" "/Game/FantasyCocktails/Assets/Back/Flipbooks/Drinks/PF_MuleDrink.PF_MuleDrink") "NewEnumerator0" "Igloo Mule" "/Game/FantasyCocktails/Assets/Back/Sprites/Drinks/SP_MuleDrink.SP_MuleDrink")
  ;[0.006732 0.2031 0] Spore Dew
  (CallFunction|NewRecipe "NewEnumerator6" (Utilities|Array|MakeArray "NewEnumerator10" "NewEnumerator16" "NewEnumerator17" "NewEnumerator3") "NewEnumerator0" "NewEnumerator5" "NewEnumerator4" (Utilities|Array|MakeArray "NewEnumerator0" "NewEnumerator1") "NewEnumerator0" (Utilities|Map|MakeMap "NewEnumerator0" "/Game/FantasyCocktails/Assets/Back/Flipbooks/Drinks/SporeDew/PF_MartiniGreen.PF_MartiniGreen" "NewEnumerator1" "/Game/FantasyCocktails/Assets/Back/Flipbooks/Drinks/SporeDew/PF_RocksGreen.PF_RocksGreen" "NewEnumerator2" "/Game/FantasyCocktails/Assets/Back/Flipbooks/Drinks/SporeDew/PF_HurricaneGreen.PF_HurricaneGreen" "NewEnumerator3" "/Game/FantasyCocktails/Assets/Back/Flipbooks/Drinks/SporeDew/PF_CollinsGreen.PF_CollinsGreen" "NewEnumerator4" "/Game/FantasyCocktails/Assets/Back/Flipbooks/Drinks/SporeDew/PF_CoupeGreen.PF_CoupeGreen" "NewEnumerator5" "/Game/FantasyCocktails/Assets/Back/Flipbooks/Drinks/PF_MuleDrink.PF_MuleDrink") "NewEnumerator1" "Spore Dew" "/Game/FantasyCocktails/Assets/Back/Sprites/Drinks/SporeDew/SP_CoupeGreen.SP_CoupeGreen")
  ;[0.1649 0.04744 0] Spring Sour
  (CallFunction|NewRecipe "NewEnumerator7" (Utilities|Array|MakeArray "NewEnumerator8" "NewEnumerator18" "NewEnumerator19" "NewEnumerator13" "NewEnumerator3") "NewEnumerator0" "NewEnumerator6" "NewEnumerator1" (Utilities|Array|MakeArray "NewEnumerator0" "NewEnumerator1") "NewEnumerator0" (Utilities|Map|MakeMap "NewEnumerator0" "/Game/FantasyCocktails/Assets/Back/Flipbooks/Drinks/SpringSour/PF_MartiniBrown.PF_MartiniBrown" "NewEnumerator1" "/Game/FantasyCocktails/Assets/Back/Flipbooks/Drinks/SpringSour/PF_RocksBrown.PF_RocksBrown" "NewEnumerator2" "/Game/FantasyCocktails/Assets/Back/Flipbooks/Drinks/SpringSour/PF_HurricaneBrown.PF_HurricaneBrown" "NewEnumerator3" "/Game/FantasyCocktails/Assets/Back/Flipbooks/Drinks/SpringSour/PF_CollinsBrown.PF_CollinsBrown" "NewEnumerator4" "/Game/FantasyCocktails/Assets/Back/Flipbooks/Drinks/SpringSour/PF_CoupeBrown.PF_CoupeBrown" "NewEnumerator5" "/Game/FantasyCocktails/Assets/Back/Flipbooks/Drinks/PF_MuleDrink.PF_MuleDrink") "NewEnumerator0" "Spring Sour" "/Game/FantasyCocktails/Assets/Back/Sprites/Drinks/SpringSour/SP_RocksBrown.SP_RocksBrown")
  ;[0 0 0] Sludge
  (CallFunction|NewRecipe "NewEnumerator2" "NewEnumerator0" "NewEnumerator0" "NewEnumerator1" "NewEnumerator0" "NewEnumerator0" "NewEnumerator0" (Utilities|Map|MakeMap "NewEnumerator0" "/Game/FantasyCocktails/Assets/Back/Flipbooks/Drinks/FrogMartini/PF_MartiniGray.PF_MartiniGray" "NewEnumerator1" "/Game/FantasyCocktails/Assets/Back/Flipbooks/Drinks/FrogMartini/PF_RocksGray.PF_RocksGray" "NewEnumerator2" "/Game/FantasyCocktails/Assets/Back/Flipbooks/Drinks/FrogMartini/PF_HurricaneGray.PF_HurricaneGray" "NewEnumerator3" "/Game/FantasyCocktails/Assets/Back/Flipbooks/Drinks/FrogMartini/PF_CollinsGray.PF_CollinsGray" "NewEnumerator4" "/Game/FantasyCocktails/Assets/Back/Flipbooks/Drinks/FrogMartini/PF_CoupeGray.PF_CoupeGray" "NewEnumerator5" "/Game/FantasyCocktails/Assets/Back/Flipbooks/Drinks/PF_MuleDrink.PF_MuleDrink") "NewEnumerator1" "Sludge"))

(event EventClicked
  (params (Player :type BP%20Player%20Object%20Reference))
  (bind _recipebookwidget (Variables|Default|GetRecipeBookWidget))
  (UserInterface|Viewport|AddtoViewport _recipebookwidget 0)
  (Default|Setup _recipebookwidget))

(fn ConstructionScript)

(fn GetRecipe
  (params (Drink :type E_Drink%20Enum :default "NewEnumerator0"))
  (bind _recipes (Variables|Default|GetRecipes))
  (bind (_value _returnvalue) (Utilities|Map|Find _recipes Drink))
  ;[1 1 1] Get recipe of drink
  (return _value _returnvalue))

(fn GetRecipes
  ;[1 1 1] Get recipes map
  (return (Variables|Default|GetRecipes)))

(fn NewRecipe
  (params (Type :type E_Drink%20Enum :default "NewEnumerator2") (ShakerIngredients :type Array%20of%20E_Ingredient%20Enums :default "NewEnumerator0") (GlassIngredients :type Array%20of%20E_Ingredient%20Enums :default "NewEnumerator0") (Garnish :type E_Garnish%20Enum :default "NewEnumerator1") (Glass :type E_Glass%20Enum :default "NewEnumerator0") (ShakerInstructions :type Array%20of%20E_Instruction%20Enums :default "NewEnumerator0") (GlassInstructions :type Array%20of%20E_Instruction%20Enums :default "NewEnumerator0") (Flipbooks :type Map%20of%20E_Glass%20Enums%20to%20Objects :default "NewEnumerator0") (Flair :type E_Flair%20Enum :default "NewEnumerator1") (RecipeName :type Name) (Picture :type Paper%20Sprite%20Object%20Reference))
  (bind _returnvalue (Game|ConstructObjectfromClass "/Game/FantasyCocktails/Core/BP_Recipe.BP_Recipe_C" ShakerIngredients GlassIngredients Garnish Glass ShakerInstructions GlassInstructions Flipbooks Flair Type RecipeName Picture))
  (Utilities|Map|Add (Variables|Default|GetRecipes) Type _returnvalue))

(fn Update
  (Sprite|SetFlipbook (Variables|Default|GetRenderComponent) (Variables|Default|GetFlipbook)))