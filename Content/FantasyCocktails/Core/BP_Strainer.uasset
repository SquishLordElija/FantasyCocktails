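; BP_Strainer is a clickable strainer for the cocktail game that applies itself to the player's shaker.
; On click it runs the parent logic, then, if the player has a shaker, calls ApplyStrainer on it and binds a Return handler to the shaker's strain delegate.
; When that delegate reports the strainer is no longer applied, Return calls Toggle to restore the strainer.
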(event Custom|Return
  (params (Apply :type Boolean))
  ;[1 1 1] "Return" strainer
  (if (not Apply)
    (CallFunction|Toggle true)))

(event EventBeginPlay
  (|CallParentFunction) ; This node is disabled and will not be called.\nDrag off pins to build functionality.
)

(event Collision|EventActorBeginOverlap
  (params (OtherActor :type Actor%20Object%20Reference))
  (|CallParentFunction OtherActor) ; This node is disabled and will not be called.\nDrag off pins to build functionality.
)

(event EventTick
  (params (DeltaSeconds :type Float%20%28single-precision%29))
  (|CallParentFunction DeltaSeconds) ; This node is disabled and will not be called.\nDrag off pins to build functionality.
)

(event EventClicked
  (params (Player :type BP%20Player%20Object%20Reference))
  (bind (_shaker _returnvalue) (Default|GetShaker Player))
  ;[1 1 1] Apply strainer to shaker
  (|CallParentFunction Player)
  (if _returnvalue
    (Default|ApplyStrainer _shaker true)
    (EventDispatchers|BindEventtoStrainDelegate _shaker (delegate Custom|Return))))

(fn ConstructionScript
  (|CallParentFunction))