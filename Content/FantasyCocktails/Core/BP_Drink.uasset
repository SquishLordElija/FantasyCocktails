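; BP_Drink is a cocktail the player can pick up and drop, carrying a type, a quality and a ticket.
; At BeginPlay it snaps garnish and flair flipbooks to sockets on its render component.
; An actor event accepts garnish actors, while flair is looked up by type in a map.
; Each slot fills only once, updating the sprite and ticket, then firing the drink-update delegate.
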(event EventBeginPlay
  (|CallParentFunction)
  (Transformation|SetWorldTransform (Variables|Default|GetGarnish) (Transformation|GetSocketTransform (Variables|Default|GetRenderComponent) "Garnish" "RTS_World") false false)
  (Transformation|SetWorldTransform (Variables|Default|GetFlair) (Transformation|GetSocketTransform (Variables|Default|GetRenderComponent) "Flair" "RTS_World") false false))

(event EventDrop
  (params (Player :type BP%20Player%20Object%20Reference))
  (Default|DropItem Player))

(event EventDrag
  (params (Player :type BP%20Player%20Object%20Reference))
  (if (not (Default|IsHoldingContainer Player))
    (Default|PickupItem Player)))

(event Event
  (params (Actor :type Actor%20Object%20Reference))
  (bind _asbp_garnish (Utilities|Casting|CastToBP_Garnish Actor))
  (CallFunction|GiveGarnish _asbp_garnish))

(fn ConstructionScript)

(fn GetTicket
  ;[1 1 1] Get ticket
  (return (Variables|Default|GetTicket)))

(fn GiveGarnish
  (params (NewGarnish :type BP%20Garnish%20Object%20Reference))
  ;[1 1 1] Add garnish to drink and ticket
  (if (not (CallFunction|HasGarnish))
    (Sprite|SetFlipbook (Variables|Default|GetGarnish) (Default|GetPlacedFlipbook NewGarnish))
    (Default|SetGarnish (Variables|Default|GetTicket) (Default|GetGarnishType NewGarnish))
    (Default|CallUpdateDrinkDelegate self)))

(fn GiveFlair
  (params (Type :type E_Flair%20Enum :default "NewEnumerator1"))
  (bind _flairs (Variables|Default|GetFlairs))
  (bind (_value _returnvalue) (Utilities|Map|Find _flairs Type))
  ;[1 1 1] Add flair to drink and ticket
  (if (not (CallFunction|HasFlair))
    (if _returnvalue
      (Sprite|SetFlipbook (Variables|Default|GetFlair) _value)
      (Default|SetFlair (Variables|Default|GetTicket) Type)
      (Default|CallUpdateDrinkDelegate self))))

(fn GetDrinkType
  ;[1 1 1] Get drink type
  (return (Variables|Default|GetDrinkType)))

(fn SetDrinkType
  (params (Type :type E_Drink%20Enum :default "NewEnumerator2"))
  (Variables|Default|SetDrinkType Type))

(fn GetQuality
  ;[1 1 1] Get quality
  (return (Variables|Default|GetQuality)))

(fn SetQuality
  (params (Quality :type E_Quality%20Enum :default "NewEnumerator0"))
  ;[1 1 1] Set quality
  (Variables|Default|SetQuality Quality))

(fn HasFlair
  ;[1 1 1] Check if ticket already has a flair
  (return (Utilities|Enum|NotEqual(Enum) (Default|GetFlair (Variables|Default|GetTicket)) "NewEnumerator1")))

(fn HasGarnish
  ;[1 1 1] Check if ticket already has a garnish
  (return (Utilities|Enum|NotEqual(Enum) (Default|GetGarnish (Variables|Default|GetTicket)) "NewEnumerator1")))