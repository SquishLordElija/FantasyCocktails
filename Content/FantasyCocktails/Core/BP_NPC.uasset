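; BP_NPC appears to be a base NPC Blueprint that provides voiceline-driven conversation and accessors for the game mode reference and NPC type.
; Conversate pulls a line from NextVoiceline, broadcasts it with the NPC through the NPCTalked delegate via Talk, then re-runs itself on a timer set to the line's duration.
; It returns true once no line is found; NextVoiceline here is a stub that always reports none.
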(fn ConstructionScript)

(fn GetGameModeRef
  ;[1 1 1] Get game mode ref
  (return (Variables|Default|GetGameModeRef)))

(fn GetNPCType
  ;[1 1 1] Get NPC type
  (return "NewEnumerator0"))

(fn Talk
  (params (Voiceline :type String))
  (Default|CallNPCTalkedDelegate self Voiceline))

(fn Conversate
  (bind (_voiceline _duration _found) (CallFunction|NextVoiceline))
  (if _found
    (CallFunction|Talk _voiceline)
    (Utilities|Time|SetTimerbyFunctionName 0 "Conversate" _duration)
    (return false)
    (else
      (return true))))

(fn NextVoiceline
  (return "" 0.0 false))