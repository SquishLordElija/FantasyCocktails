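; Barmaid NPC that runs the tutorial conversation, starting it automatically on BeginPlay.
; Delegates announce the tutorial's start and, when the parent's conversation ends, its end.
; NextVoiceline steps through the enum-keyed Voicelines map in key order, tracking the last line, with one sentinel value restarting at the first enum entry.
; Talk defers to the parent, and GetNPCType returns a fixed type.
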(event Custom|BeginTutorial
  (Default|CallTutorialBeganDelegate)
  (CallFunction|Conversate))

(event EventBeginPlay
  (|CallParentFunction)
  (CallFunction|BeginTutorial))

(event EventConversationEnded
  (|CallParentFunction)
  (Default|CallTutorialEndedDelegate))

(fn ConstructionScript
  (|CallParentFunction))

(fn GetVoiceline
  (params (Key :type E_BarmaidVoiceline%20Enum :default "NewEnumerator1"))
  (bind _voicelines (Variables|Default|GetVoicelines))
  (bind (_value _returnvalue) (Utilities|Map|Find _voicelines Key))
  ;[1 1 1] Get voiceline from key
  (return _value _returnvalue))

(fn GetNPCType
  ;[1 1 1] Get NPC type
  (return "NewEnumerator1"))

(fn NextVoiceline
  (if (Utilities|Enum|NotEqual(Enum) (Variables|Default|GetLastVoiceline) (Utilities|Enum|LiteralenumE_BarmaidVoiceline "NewEnumerator1"))
    (bind _keys (Utilities|Map|Keys (Variables|Default|GetVoicelines)))
    (for _array_element _keys
      (if (LocalVariables|GetLastVoicelineFound)
        (bind _output_get (Variables|Default|SetLastVoiceline _array_element))
        (return (.Voiceline (CallFunction|GetVoiceline _output_get)) (.Found (CallFunction|GetVoiceline _output_get)))
        (else
          (LocalVariables|SetLastVoicelineFound (Utilities|Enum|Equal(Enum) _array_element (Variables|Default|GetLastVoiceline))))))
    (return "" false)
    (else
      (bind _output_get_2 (Variables|Default|SetLastVoiceline "NewEnumerator0"))
      (return (.Voiceline (CallFunction|GetVoiceline _output_get_2)) (.Found (CallFunction|GetVoiceline _output_get_2))))))

(fn Talk
  (params (Voiceline :type F%20Voiceline%20Structure))
  (|CallParentFunction Voiceline))