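; BP_Queue is a placeable queue spot that tracks whether it is occupied.
; GetLocation returns the spot's world position by adding its Location offset to the actor's location, without applying actor rotation.
; Occupy and Vacate set the Occupied flag, which IsOccupied reports.
; It runs no event or construction logic, so other code drives it entirely through these functions.
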(event EventBeginPlay)

(event Collision|EventActorBeginOverlap
  (params (OtherActor :type Actor%20Object%20Reference)))

(event EventTick
  (params (DeltaSeconds :type Float%20%28single-precision%29)))

(fn ConstructionScript)

(fn GetLocation
  ;[1 1 1] Get location
  (return (+ (Variables|Default|GetLocation) (Transformation|GetActorLocation))))

(fn IsOccupied
  ;[1 1 1] Get occupied
  (return (Variables|Default|GetOccupied)))

(fn Occupy
  (Variables|Default|SetOccupied true))

(fn Vacate
  (Variables|Default|SetOccupied false))