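; Base Paper2D container actor for a cocktail-mixing game, tracking the ingredients added and the instructions completed on it, such as shake and strain.
; Functions add or query contents, empty them, and swap the flipbook.
; GetMeta turns both lists into one array of display strings.
; Reset restores the transform and translucency sort priority cached at BeginPlay, leaving contents intact, while GetContainerType and GetName return placeholder defaults.
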(event EventBeginPlay
  (Variables|Default|SetDefaultTransform (Transformation|GetActorTransform))
  (Variables|Default|SetDefaultTranslucencyPriority (Variables|/Script/Engine.PrimitiveComponent|GetTranslucencySortPriority (Variables|Default|GetRenderComponent))))

(event EventClicked
  (params (Player :type BP%20Player%20Object%20Reference)))

(event EventTick
  (params (DeltaSeconds :type Float%20%28single-precision%29)))

(event Event
  (params (Actor :type Actor%20Object%20Reference))
  (Audio|PlaySound2D "/Game/FantasyCocktails/Sounds/SFX_GlassTing.SFX_GlassTing" 1.0 1.0 0.0 0 0))

(fn ConstructionScript)

(fn GetIngredients
  (return (Variables|Default|GetIngredients)))

(fn AddIngredient
  (params (Ingredient :type E_Ingredient%20Enum :default "NewEnumerator0"))
  (Utilities|Array|Add (Variables|Default|GetIngredients) Ingredient)
  (return Ingredient))

(fn GetInstructions
  ;[1 1 1] Get instructions
  (return (Variables|Default|GetInstructions)))

(fn CompleteInstruction
  (params (Instruction :type E_Instruction%20Enum :default "NewEnumerator0"))
  (Utilities|Array|Add (Variables|Default|GetInstructions) Instruction))

(fn Empty
  (Utilities|Array|Clear (Variables|Default|GetIngredients))
  (Utilities|Array|Clear (Variables|Default|GetInstructions)))

(fn UpdateFlipbook
  (params (Flipbook :type Paper%20Flipbook%20Object%20Reference))
  ;[1 1 1] Update flipbook
  (Sprite|SetFlipbook (Variables|Default|GetRenderComponent) Flipbook))

(fn Reset
  (Transformation|SetActorTransform (Variables|Default|GetDefaultTransform))
  (Rendering|SetTranslucentSortPriority (Variables|Default|GetRenderComponent) (Variables|Default|GetDefaultTranslucencyPriority)))

(fn GetContainerType
  (return "NewEnumerator0"))

(fn HasCompletedInstruction
  (params (Instruction :type E_Instruction%20Enum :default "NewEnumerator0"))
  ;[1 1 1] Return if instruction has been completed
  (return (Utilities|Array|ContainsItem (CallFunction|GetInstructions) Instruction)))

(fn RemoveInstruction
  (params (Instruction :type E_Instruction%20Enum :default "NewEnumerator0"))
  (bind _instructions (Variables|Default|GetInstructions))
  (if (Utilities|Array|ContainsItem _instructions Instruction)
    (Utilities|Array|RemoveIndex (Variables|Default|GetInstructions) (Utilities|Array|FindItem _instructions Instruction))))

(fn GetMeta
  (for _array_element (CallFunction|GetIngredients)
    (Utilities|Array|Add (LocalVariables|GetIngredientsMeta) (|GetIngredientName _array_element)))
  (for _array_element_2 (CallFunction|GetInstructions)
    (Utilities|Array|Add (LocalVariables|GetInstructionsMeta) (Utilities|Select :Index _array_element_2 :NewEnumerator0 (Utilities|String|MakeLiteralString "Shaken") :NewEnumerator1 (Utilities|String|MakeLiteralString "Strained"))))
  (Utilities|Array|AppendArray (LocalVariables|GetIngredientsMeta) (LocalVariables|GetInstructionsMeta))
  (return (LocalVariables|GetIngredientsMeta)))

(fn GetName
  (return ""))