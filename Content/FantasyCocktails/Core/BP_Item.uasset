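; Item actor for FantasyCocktails that displays a Paper2D flipbook.
; On BeginPlay it caches its spawn transform as DefaultTransform and exposes it through a getter.
; Update applies PrimaryFlipbook to the render component, and a second getter returns that flipbook.
; Update is not called within this Blueprint, and the construction script is empty.
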(event EventBeginPlay
  (Variables|Default|SetDefaultTransform (Transformation|GetActorTransform)))

(fn ConstructionScript)

(fn Update
  (Sprite|SetFlipbook (Variables|Default|GetRenderComponent) (Variables|Default|GetPrimaryFlipbook)))

(fn GetDefaultTransform
  (return (Variables|Default|GetDefaultTransform)))

(fn GetPrimaryFlipbook
  ;[1 1 1] Get flipbook
  (return (Variables|Default|GetPrimaryFlipbook)))