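; BP_ItemManager is a manager for the glasses, garnishes and ingredients placed in a cocktail-making level.
; Lookup functions search per-category maps by type, returning the matching item and a found flag.
; It also tracks the active glass, teleport-free moving a newly assigned one to a stored transform without sweep, and reports whether one is valid.
; The file only reads the maps and contains no code that fills them.
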(event EventBeginPlay)

(fn ConstructionScript)

(fn GetGlass
  (params (Type :type E_Glass%20Enum%20%28by%20ref%29 :default "NewEnumerator0"))
  (bind _glasses (Variables|Items|GetGlasses))
  (bind (_value _returnvalue) (Utilities|Map|Find _glasses Type))
  ;[1 1 1] Get glass in level from type
  (return _value _returnvalue))

(fn GetGarnish
  (params (Type :type E_Garnish%20Enum%20%28by%20ref%29 :default "NewEnumerator0"))
  (bind _garnishes (Variables|Items|GetGarnishes))
  (bind (_value _returnvalue) (Utilities|Map|Find _garnishes Type))
  ;[1 1 1] Get garnish in level from type
  (return _value _returnvalue))

(fn GetIngredient
  (params (Type :type E_Ingredient%20Enum%20%28by%20ref%29 :default "NewEnumerator0"))
  (bind _ingredients (Variables|Items|GetIngredients))
  (bind (_value _returnvalue) (Utilities|Map|Find _ingredients Type))
  ;[1 1 1] Get ingredient in level from type
  (return _value _returnvalue))

(fn GetActiveGlass
  (return (Variables|Default|GetActiveGlass)))

(fn UpdateActiveGlass
  (params (Glass :type BP%20Glass%20Object%20Reference))
  (bind _output_get (Variables|Default|SetActiveGlass Glass))
  (Transformation|SetActorTransform _output_get (Variables|Default|GetActiveGlassTransform)))

(fn IsActiveGlass
  (return (Utilities|IsValid (Variables|Default|GetActiveGlass))))